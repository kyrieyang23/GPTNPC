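; Game mode that runs voice conversations with an AI NPC and shows both sides in a dialogue widget.
; NPCTalk chains speech-to-text, a GPT-3 completion and text-to-speech, with IsProcess blocking new requests until the reply ends.
; Each exchange is appended to StartSequence as conversation memory, and IsTalking stays true for a delay estimated from reply length.
; BeginPlay creates the widget and sets a hardcoded OpenAI API key.
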(event `self.ReceiveBeginPlay`
  (`OpenAIUtils.setOpenAIApiKey` "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")
  (bind _returnvalue (`|CreateWidget` "/Game/Widget/DialougeWidget.DialougeWidget_C"))
  (bind _output_get (set `self.DialougeWidget` _returnvalue))
  (`UserWidget.AddToViewport` _output_get 0))

(event `NPCTalk`
  (if (not (`self.IsProcess`))
    (bind (_asynctaskproxy _finalstring) (`SpeechToTextAsync.SpeechToText_DefaultOptions` "Default")
      (:`RecognitionCompleted`
        (if (> (`KismetStringLibrary.Len` _finalstring) 0)
          (`/Game/Widget/DialougeWidget.ChangeDialouge` (`self.DialougeWidget`) (`KismetStringLibrary.Concat_StrStr` "You: " _finalstring))
          (set `self.IsProcess` true)
          (bind (_completions _errormessage _completioninfo _success) (`OpenAICallGPT.OpenAICallGPT3` "TEXT_DAVINCI_003" _finalstring (make `GPT3Settings` (`self.Start Sequence`) "AI:" "" (`self.Stop Sequences`) 150 0.9 1.0 0 1 0.6 0.0 4))
            (:`Finished`
              (if _success
                (for _array_element _completions
                  (bind _text (break `Completion` _array_element))
                  (set `self.Start Sequence` (`KismetStringLibrary.Concat_StrStr` (`self.Start Sequence`) _finalstring " \nAI:" _text " \nHuman:"))
                  (`TextToSpeechAsync.TextToSpeech` _text
                    (:`SynthesisCompleted`
                      (bind _returnvalue (`KismetStringLibrary.Replace` (`KismetStringLibrary.Concat_StrStr` "NPC: " _text) (`KismetStringLibrary.Right` " \n" 1)))
                      (`/Game/Widget/DialougeWidget.ChangeDialouge` (`self.DialougeWidget`) _returnvalue)
                      (set `self.IsTalking` true)
                      (`KismetSystemLibrary.Delay` (`KismetMathLibrary.Conv_IntToDouble` (/ (`KismetStringLibrary.Len` _returnvalue) 13)))
                      (set `self.IsTalking` false)
                      (set `self.IsProcess` false)
                      (`/Game/Widget/DialougeWidget.ChangeDialouge` (`self.DialougeWidget`) ""))))))))))))

(fn `UserConstructionScript`)